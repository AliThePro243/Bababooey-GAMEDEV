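; Child Blueprint of a shooter enemy AI that sets its health on BeginPlay and configures its weapon loadout.
; The WeaponSetup override calls the parent, then switches on the weapon type: assault rifle, machine gun or sniper rifle.
; Each branch swaps and positions the weapon mesh and sets fire sound, rate, damage, ammo, recoil, aim time and reload animation.
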(event `self.ReceiveBeginPlay`
  (`parent.ReceiveBeginPlay`)
  (set `self.EnemyHP` 100.0))

(fn `UserConstructionScript`
  (`parent.UserConstructionScript`))

(fn `Weapon Setup`
  (bind _weapon (`self.Weapon`))
  (bind _weapon_2 (`self.Weapon`))
  (bind _weapon_3 (`self.Weapon`))
  (`parent.Weapon Setup`)
  (switch `/Game/ShooterSimplifiedAI/Blueprints/AI/E_AI_WeaponType` (`self.AIWeponTypes`)
    (:`NewEnumerator0`
      ;[1 1 1] AssaultRifle
      (`SceneComponent.SetWorldScale3D` _weapon_3 (1.0 1.0 1.0))
      (`SceneComponent.K2_SetRelativeLocationAndRotation` :`self` _weapon_3 :`NewLocation` (-2.0 -28.0 -4.0))
      (`SkinnedMeshComponent.SetSkinnedAssetAndUpdate` _weapon_3 "/Game/ShooterSimplifiedAI/Weapons/AssaultRifle/Mesh/AssaultRifle.AssaultRifle" true)
      (set `self.WeaponSound` "/Game/ShooterSimplifiedAI/Audio/SC_WeaponFire_Cue.SC_WeaponFire_Cue")
      (set `self.WeaponFireRate` 0.5)
      (set `self.WeaponDamage` 3.0)
      (bind _output_get (set `self.MaxAmmo` 10))
      (set `self.AmmoInMag` _output_get)
      (set `self.WeaponRecoil` 10.0)
      (set `self.WeaponAimTime` 0.3)
      (set `self.ReloadAnimPlayRate` 1.0)
      (set `self.WeaponReloadMontage` "/Game/ShooterSimplifiedAI/Animations/AM_Reload_Rifle_Ironsights.AM_Reload_Rifle_Ironsights"))
    (:`NewEnumerator1`
      ;[1 1 1] Machine Gun
      (`SceneComponent.SetWorldScale3D` _weapon_2 (1.0 1.0 1.0))
      (`SceneComponent.K2_SetRelativeLocationAndRotation` _weapon_2 (-0.9 15.0 11.0) (struct :`Yaw` -2.0) false false)
      (`SkinnedMeshComponent.SetSkinnedAssetAndUpdate` _weapon_2 "/Game/ShooterSimplifiedAI/Weapons/MachineGun/Mesh/SM_MachineGun.SM_MachineGun" true)
      (set `self.WeaponSound` "/Game/ShooterSimplifiedAI/Audio/SC_WeaponFire_Cue.SC_WeaponFire_Cue")
      (set `self.WeaponFireRate` 0.2)
      (set `self.WeaponDamage` 1.0)
      (bind _output_get_2 (set `self.MaxAmmo` 15))
      (set `self.AmmoInMag` _output_get_2)
      (set `self.WeaponRecoil` 20.0)
      (set `self.WeaponAimTime` 0.5)
      (set `self.ReloadAnimPlayRate` 0.8)
      (set `self.WeaponReloadMontage` "/Game/ShooterSimplifiedAI/Animations/AM_Reload_Rifle_Ironsights.AM_Reload_Rifle_Ironsights"))
    (:`NewEnumerator2`
      ;[1 1 1] Sniper Rifle
      (`SceneComponent.SetWorldScale3D` _weapon (0.11 0.11 0.11))
      (`SceneComponent.K2_SetRelativeLocationAndRotation` _weapon (-0.907428 3.833228 -7.0) (struct :`Yaw` 94.0) false false)
      (`SkinnedMeshComponent.SetSkinnedAssetAndUpdate` _weapon "/Game/ShooterSimplifiedAI/Weapons/SniperRifle/Mesh/SM_SniperRifle.SM_SniperRifle" true)
      (set `self.WeaponSound` "/Game/ShooterSimplifiedAI/Audio/SC_WeaponFire_Cue.SC_WeaponFire_Cue")
      (set `self.WeaponFireRate` 3.0)
      (set `self.WeaponDamage` 15.0)
      (bind _output_get_3 (set `self.MaxAmmo` 1))
      (set `self.AmmoInMag` _output_get_3)
      (set `self.WeaponRecoil` 5.0)
      (set `self.WeaponAimTime` 1.0)
      (set `self.ReloadAnimPlayRate` 0.8)
      (set `self.WeaponReloadMontage` "/Game/ShooterSimplifiedAI/Animations/AM_Reload_Rifle_Ironsights.AM_Reload_Rifle_Ironsights"))))